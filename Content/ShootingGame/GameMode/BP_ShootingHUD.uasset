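; BP_ShootingHUD is the shooting game's HUD Blueprint, which passes player HP, ammo and magazine updates on to its on-screen widget.
; Each update event casts HudWidget to ShootingHudWidget and does nothing further if the cast fails.
; HP and ammo go through the widget's setter functions, while the magazine value is written straight to its Mag variable.
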(event EventOnUpdateMyAmmo
  (params (Ammo :type Integer))
  (bind _asshooting_hud_widget (Utilities|Casting|CastToShootingHudWidget (Variables|Default|GetHudWidget)))
  (Default|SetAmmo _asshooting_hud_widget Ammo))

(event EventOnUpdateMyMag
  (params (Mag :type Integer))
  (bind _asshooting_hud_widget (Utilities|Casting|CastToShootingHudWidget (Variables|Default|GetHudWidget)))
  (Variables|/Game/ShootingGame/Widget/ShootingHudWidget.ShootingHudWidget_C|SetMag _asshooting_hud_widget Mag))

(event EventOnUpdateMyHP
  (params (CurHP :type Float%20%28single-precision%29) (MaxHP :type Float%20%28single-precision%29))
  (bind _asshooting_hud_widget (Utilities|Casting|CastToShootingHudWidget (Variables|Default|GetHudWidget)))
  (Default|SetHP _asshooting_hud_widget CurHP MaxHP))

(fn ConstructionScript)